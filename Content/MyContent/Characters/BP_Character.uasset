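; Networked shooter character with movement, camera, jumping, aim-down-sights and a starter weapon.
; The weapon is a child actor fired on trigger change, supplying a left-hand IK transform relative to hand_r.
; Tick interpolates spring arm length for aim zoom and draws debug health.
; Point damage reduces stats-component health, restarting the player at zero, while control rotation replicates through a server event only when pitch drifts past a tolerance.
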(event `self.ReceiveTick`
  (params (DeltaSeconds :type "Float (single-precision)"))
  (`self.HandleZoom`)
  (`KismetSystemLibrary.DrawDebugString` (+ (`self.GetActorEyesViewPoint`) (0.0 0.0 50.0)) (`KismetStringLibrary.Conv_IntToString` (`/Game/MyContent/Core/BP_StatsComponent.GetHealth` (`self.BP_StatsComponent`))) null (struct :`R` 1.0 :`A` 1.0)))

(event `Server_UpdateRepControlRotation`
  (params (Rotation :type "Rotator Structure"))
  (set `self.RepControlRotation` Rotation))

(event `self.OnTriggerChanged`
  (params (pullOrRelease :type Boolean))
  (if true
    (bind _asbp_weapon (cast `/Game/MyContent/Weapons/BP_Weapon` (`ChildActorComponent.ChildActor` (`self.WeaponActorComponent`))))
    (`/Game/MyContent/Weapons/BP_Weapon.Fire` _asbp_weapon)))

(event `self.ReceivePointDamage`
  (params (Damage :type "Float (single-precision)") (DamageType :type "DamageType Object Reference") (HitLocation :type "Vector Structure") (HitNormal :type "Vector Structure") (HitComponent :type "PrimitiveComponent Object Reference") (BoneName :type Name) (ShotFromDirection :type "Vector Structure") (InstigatedBy :type "Controller Object Reference") (DamageCauser :type "Actor Object Reference") (HitInfo :type "HitResult Structure (by ref)"))
  (bind _returnvalue (`self.GetController`))
  (bind _health (`/Game/MyContent/Core/BP_StatsComponent.GetHealth` (`self.BP_StatsComponent`)))
  (if (> _health 0)
    (`/Game/MyContent/Core/BP_StatsComponent.SetHealth` (`self.BP_StatsComponent`) (- _health (`KismetMathLibrary.FTrunc` Damage)))
    (if (<= (`/Game/MyContent/Core/BP_StatsComponent.GetHealth` (`self.BP_StatsComponent`)) 0)
      (`Controller.UnPossess` _returnvalue)
      (`GameModeBase.RestartPlayer` (`GameplayStatics.GetGameMode`) _returnvalue))))

(event `SetHealthTarget`
  (params (`Target  Actor` :type "Actor Object Reference"))
  (`/Engine/EditorBlueprintResources/StandardMacros.IsValid` (`self.GetComponentByClass` `Target  Actor` "/Game/MyContent/Core/BP_StatsComponent.BP_StatsComponent_C")
    (:`Is Valid`
      (bind _output_get (set `self.Target  Actor` `Target  Actor`))
      (`self.OnHealthTragetChanged` _output_get))))

(fn `ActivateWeapon`
  (params (WeaponClass :type "/Game/MyContent/Weapons/BP_Weapon Class Reference"))
  (`ChildActorComponent.SetChildActorClass` (`self.WeaponActorComponent`) WeaponClass)
  (bind _asbp_weapon (cast `/Game/MyContent/Weapons/BP_Weapon` (`ChildActorComponent.ChildActor` (`self.WeaponActorComponent`))))
  (`/Game/MyContent/Weapons/BP_Weapon.InitWeapon` _asbp_weapon self))

(fn `AimDownSights`
  (params (Enable :type Boolean))
  (set `self.IsAiming` Enable)
  (set `self.CameraZoom` (`KismetMathLibrary.SelectFloat` (`self.ZoomAim`) (`self.ZoomDefault`) Enable)))

(fn `GetAimInformation`
  (returns (ShootLocation :type "Vector Structure") (ShootDirection :type "Vector Structure"))
  (bind _camera (`self.Camera`))
  (return (`SceneComponent.K2_GetComponentLocation` _camera) (`SceneComponent.GetForwardVector` _camera)))

(fn `GetWeaponIK`
  (returns (ReturnValue :type "Transform Structure"))
  (bind _childactor (`ChildActorComponent.ChildActor` (`self.WeaponActorComponent`))
    (:`then`
      (bind _asbp_weapon (cast `/Game/MyContent/Weapons/BP_Weapon` _childactor))
      (bind (_returnvalue_location _returnvalue_rotation) (`KismetMathLibrary.BreakTransform` (`SceneComponent.GetSocketTransform` (`/Game/MyContent/Weapons/BP_Weapon.SKM_Weapon` _asbp_weapon) "hand_l_ik" "RTS_World")))
      (bind (_outposition _outrotation) (`SkinnedMeshComponent.TransformToBoneSpace` (`self.Mesh`) "hand_r" _returnvalue_location _returnvalue_rotation))
      (return (`KismetMathLibrary.MakeTransform` _outposition _outrotation)))
    (:`else`)))

(fn `HandleZoom`
  (if (not (`KismetMathLibrary.NearlyEqual_FloatFloat` (`self.CameraZoom`) (`SpringArmComponent.TargetArmLength` (`self.SpringArm`)) 0.01))
    (set `SpringArmComponent.TargetArmLength` (`KismetMathLibrary.FInterpTo` (`SpringArmComponent.TargetArmLength` (`self.SpringArm`)) (`self.CameraZoom`) (`GameplayStatics.GetWorldDeltaSeconds`) 10.0) (`self.SpringArm`))))

(fn `MoveCharacter`
  (params (Axis :type "Vector2D Structure"))
  (bind _output_get (set `self.MoveAxis` Axis))
  (`self.PMoveCharacter` (`KismetMathLibrary.MakeVector2D` (`KismetMathLibrary.BreakVector2D` _output_get) (`.Y` (`KismetMathLibrary.BreakVector2D` _output_get)))))

(fn `RotateCamera`
  (params (Axis :type "Vector2D Structure"))
  (bind (_returnvalue_roll _returnvalue_pitch) (`KismetMathLibrary.BreakRotator` (`self.GetControlRotation`)))
  (bind (_repcontrolrotation_roll _repcontrolrotation_pitch) (`KismetMathLibrary.BreakRotator` (`self.RepControlRotation`)))
  (`self.AddControllerYawInput` Axis_X)
  (`self.AddControllerPitchInput` (* Axis_Y -1.0))
  (if (not (`KismetMathLibrary.NearlyEqual_FloatFloat` _repcontrolrotation_pitch _returnvalue_pitch 10.0))
    (`/Engine/EditorBlueprintResources/ActorMacros.Switch Has Authority`
      (:`Authority`
        (set `self.RepControlRotation` (`self.GetControlRotation`)))
      (:`Remote`
        (`self.Server_UpdateRepControlRotation` (`self.GetControlRotation`))))))

(fn `TryJump`
  (params (`Jump/Stop` :type Boolean))
  (if `Jump/Stop`
    (`self.Jump`)
    (else
      (`self.StopJumping`))))

(fn `UserConstructionScript`
  (`self.ActivateWeapon` (`self.StarterWeapon`))
  (set `self.CameraZoom` (`self.ZoomDefault`)))