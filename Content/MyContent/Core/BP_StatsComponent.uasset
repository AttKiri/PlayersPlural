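; BP_StatsComponent is a stats component that holds Health and MaxHealth, exposed through setters and a combined getter.
; SetHealth clamps Health between zero and MaxHealth, while SetMaxHealth only floors MaxHealth at zero without re-clamping Health.
; Both setters and both RepNotify functions fire the OnHealthChange dispatcher, so listeners hear local and replicated changes alike.
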(fn `GetHealth`
  (returns (Health :type Integer) (MaxHealth :type Integer))
  (return (`self.Health`) (`self.MaxHealth`)))

(fn `OnRep_Health`
  (`self.OnHealthChange`))

(fn `OnRep_MaxHealth`
  (`self.OnHealthChange`))

(fn `SetHealth`
  (params (Health :type Integer))
  (set `self.Health` (`KismetMathLibrary.Clamp` Health 0 (`self.MaxHealth`)))
  (`self.OnHealthChange`))

(fn `SetMaxHealth`
  (params (MaxHealth :type Integer))
  (set `self.MaxHealth` (`KismetMathLibrary.Max` MaxHealth))
  (`self.OnHealthChange`))